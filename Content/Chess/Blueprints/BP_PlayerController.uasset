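; Player controller for the chess game that turns mouse and key input into piece selection, moves and camera rotation, passed to BP_GameMode.
; Cursor object traces find board squares and pieces; clicking an opposing piece selects its square instead, and selection and move input can be disabled.
; It also creates the main HUD, refreshing it from game mode state with check and end-game messages, and opens the restart menu.
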(event `InputAction|MoveChessPiece`
  (params (Key :type "Key Structure"))
  (:`Pressed`
    (if (`self.InputsEnabled`)
      (`/Game/Chess/Blueprints/BP_GameMode.ProcessMove` (`self.GameModeRef`)))))

(event `InputAxis|RotatePlayerCamera`
  (params (AxisValue :type "Float (single-precision)"))
  (`/Game/Chess/Blueprints/BP_GameMode.RotateCamera` (`self.GameModeRef`) AxisValue))

(event `InputAction|OpenRestartMenu`
  (params (Key :type "Key Structure"))
  (:`Pressed`
    (`self.OpenRestartMenu`)))

(event `InputAction|FreeLook`
  (params (Key :type "Key Structure"))
  (:`Pressed`
    (set `self.CanFreeLook` true))
  (:`Released`
    (set `self.CanFreeLook` false)))

(event `InputAxis|RotatePlayerUp`
  (params (AxisValue :type "Float (single-precision)"))
  (bind _azimuth (`/Game/Chess/Blueprints/BP_Player.Azimuth` (`/Game/Chess/Blueprints/BP_GameMode.PlayerRef` (`self.GameModeRef`))))
  (bind (_relativerotation_roll _relativerotation_pitch _relativerotation_yaw) (`KismetMathLibrary.BreakRotator` (`SceneComponent.RelativeRotation` _azimuth)))
  (if (!= AxisValue 0.0)
    (`SceneComponent.K2_SetRelativeRotation` _azimuth (`KismetMathLibrary.MakeRotator` (+ AxisValue _relativerotation_roll) _relativerotation_pitch _relativerotation_yaw) false false)))

(event `InputAxis|RotateRightMouse`
  (params (AxisValue :type "Float (single-precision)"))
  (bind _azimuth (`/Game/Chess/Blueprints/BP_Player.Azimuth` (`/Game/Chess/Blueprints/BP_GameMode.PlayerRef` (`self.GameModeRef`))))
  (bind (_relativerotation_roll _relativerotation_pitch _relativerotation_yaw) (`KismetMathLibrary.BreakRotator` (`SceneComponent.RelativeRotation` _azimuth)))
  (if (`self.CanFreeLook`)
    (`SceneComponent.K2_SetRelativeRotation` _azimuth (`KismetMathLibrary.MakeRotator` _relativerotation_roll _relativerotation_pitch (* (+ AxisValue _relativerotation_yaw) 1.0)) false false)))

(event `InputAxis|RotateUpMouse`
  (params (AxisValue :type "Float (single-precision)"))
  (bind _azimuth (`/Game/Chess/Blueprints/BP_Player.Azimuth` (`/Game/Chess/Blueprints/BP_GameMode.PlayerRef` (`self.GameModeRef`))))
  (bind (_relativerotation_roll _relativerotation_pitch _relativerotation_yaw) (`KismetMathLibrary.BreakRotator` (`SceneComponent.RelativeRotation` _azimuth)))
  (if (`self.CanFreeLook`)
    (`SceneComponent.K2_SetRelativeRotation` _azimuth (`KismetMathLibrary.MakeRotator` (* (+ AxisValue _relativerotation_roll) 1.0) _relativerotation_pitch _relativerotation_yaw) false false)))

(event `InputAction|SelectSquare`
  (params (Key :type "Key Structure"))
  ;[1 1 1] SelectSquare
  (:`Pressed`
    (if (`self.InputsEnabled`)
      (bind (_selectedsquare _isvalid) (`self.GetSquareUnderCursor`))
      (if _isvalid
        (bind (_positionx _positiony) (`/Game/Chess/Blueprints/Board/BP_BoardSquare.GetSquareCoordinates` _selectedsquare))
        (`/Game/Chess/Blueprints/BP_GameMode.SelectSquare` (`self.GameModeRef`) _positionx _positiony)))))

(event `InputAction|SelectPiece`
  (params (Key :type "Key Structure"))
  (bind _gamemoderef (`self.GameModeRef`))
  ;[1 1 1] Select Piece
  (:`Pressed`
    (if (`self.InputsEnabled`)
      (bind (_selectedpiece _isvalid) (`self.GetPieceUnderCursor`))
      (if _isvalid
        (if (`|EnumEquality` (`/Game/Chess/Blueprints/ChessPieces/BP_ChessPiece.Get Piece Color` _selectedpiece) (`/Game/Chess/Blueprints/BP_GameMode.GetActivePlayerColor` (`self.GameModeRef`)))
          (`/Game/Chess/Blueprints/BP_GameMode.SelectPiece` _gamemoderef _selectedpiece)
          (else
            (`/Game/Chess/Blueprints/Board/BP_Board.SelectSquare` (`/Game/Chess/Blueprints/BP_GameMode.BoardRef` _gamemoderef) (`/Game/Chess/Blueprints/ChessPieces/BP_ChessPiece.X` _selectedpiece) (`/Game/Chess/Blueprints/ChessPieces/BP_ChessPiece.Y` _selectedpiece))))))))

(fn `CheckForEnPassant`)

(fn `DisableInputs`
  (set `self.InputsEnabled` false)
  (return))

(fn `DisplayMessgaeBaseOnEndGame`
  (locals (EndGameMessage :type String))
  (switch `/Game/Chess/Blueprints/EN_EndGameStatus` (`/Game/Chess/Blueprints/BP_GameMode.GetEndGameStatus` (`self.GameModeRef`))
    (:`NewEnumerator0`
      (set `local.EndGameMessage` ""))
    (:`NewEnumerator1`
      (set `local.EndGameMessage` "DRAW! Insufficient Material!"))
    (:`NewEnumerator2`
      (set `local.EndGameMessage` "DRAW! Threefold Repetition"))
    (:`NewEnumerator3`
      (set `local.EndGameMessage` "DRAW!  50 Move Rule!"))
    (:`NewEnumerator4`
      (set `local.EndGameMessage` "Check Mate! Game Over!"))
    (:`NewEnumerator5`
      (set `local.EndGameMessage` "DRAW!  Stalemate!"))
    (:`NewEnumerator6`
      (set `local.EndGameMessage` "Resignation! Game Over!"))
    (:`NewEnumerator7`
      (set `local.EndGameMessage` "DRAW!  Draw offer accepted!")))
  (`/Game/Chess/UI/UI_Main.SetMessage2` (`self.MainUIRef`) (`local.EndGameMessage`)))

(fn `EnableInputs`
  (set `self.InputsEnabled` true)
  (return))

(fn `GetPieceUnderCursor`
  (returns (SelectedPiece :type "/Game/Chess/Blueprints/ChessPieces/BP_ChessPiece Object Reference") (IsValid :type Boolean))
  (bind (_hitresult _returnvalue) (`self.GetHitResultUnderCursorForObjects` (`|MakeArray` "ObjectTypeQuery8" :!type "EObjectTypeQuery Enum")))
  (if _returnvalue
    (bind _asbp_chess_piece (cast `/Game/Chess/Blueprints/ChessPieces/BP_ChessPiece` (`.HitActor` (`GameplayStatics.BreakHitResult` _hitresult)))
      (:`then`
        (return _asbp_chess_piece true))
      (:`CastFailed`
        _)))
  (return null false))

(fn `GetSquareUnderCursor`
  (returns (SelectedSquare :type "/Game/Chess/Blueprints/Board/BP_BoardSquare Object Reference") (IsValid :type Boolean))
  (bind (_hitresult _returnvalue) (`self.GetHitResultUnderCursorForObjects` (`|MakeArray` "ObjectTypeQuery7" :!type "EObjectTypeQuery Enum")))
  (if _returnvalue
    (bind _asbp_board_square (cast `/Game/Chess/Blueprints/Board/BP_BoardSquare` (`.HitActor` (`GameplayStatics.BreakHitResult` _hitresult)))
      (:`then`
        (return _asbp_board_square true))
      (:`CastFailed`
        _)))
  (return null false))

(fn `Initialize`
  (`self.SetGameModeRef`)
  (set `self.bShowMouseCursor` true)
  (return))

(fn `OpenRestartMenu`
  (bind _returnvalue (`|CreateWidget` "/Game/Chess/UI/RestartMenu.RestartMenu_C" self))
  (bind _output_get (set `self.RestartMenuRef` _returnvalue))
  (`UserWidget.AddToViewport` _output_get 0)
  (`WidgetBlueprintLibrary.SetInputMode_UIOnlyEx` self (`self.RestartMenuRef`)))

(fn `SetGameModeRef`
  (`/Engine/EditorBlueprintResources/StandardMacros.IsValid` (`self.GameModeRef`)
    (:`Is Not Valid`
      (bind _asbp_game_mode (cast `/Game/Chess/Blueprints/BP_GameMode` (`GameplayStatics.GetGameMode`)))
      (set `self.GameModeRef` _asbp_game_mode))))

(fn `SetMainUI`
  (bind _returnvalue (`|CreateWidget` "/Game/Chess/UI/UI_Main.UI_Main_C" self))
  (bind _output_get (set `self.MainUIRef` _returnvalue))
  (`UserWidget.AddToViewport` _output_get 0)
  (`/Game/Chess/UI/UI_Main.OpenUI` (`self.MainUIRef`))
  (`self.UpdateUI`)
  (return))

(fn `SetMessage`
  (params (NewMessage :type String)))

(fn `SetPlayerInfoInUI`
  (params (PlayerIndex :type Integer))
  (bind (_name _color _index _kingincheck _haslegalmovesflag _movecount _captures) (break `/Game/Chess/Blueprints/ST_Player` (`/Game/Chess/Blueprints/BP_GameMode.GetPlayerByIndex` (`self.GameModeRef`) PlayerIndex)))
  (`/Game/Chess/UI/UI_Main.SetPlayerName` (`self.MainUIRef`) _color _name)
  (`/Game/Chess/UI/UI_Main.SetCheckStatus` (`self.MainUIRef`) _color _kingincheck)
  (`/Game/Chess/UI/UI_Main.SetCaptureCounts` (`self.MainUIRef`) _color _captures))

(fn `UpdateUI`
  (bind (_color _latestmovenotation) (`/Game/Chess/Blueprints/BP_GameMode.GetLatestMove` (`self.GameModeRef`)))
  (`/Game/Chess/UI/UI_Main.SetActivePlayer` (`self.MainUIRef`) (`/Game/Chess/Blueprints/BP_GameMode.GetActivePlayerColor` (`self.GameModeRef`)))
  (`|ExecutionSequence`
    (:`then_1`
      (`/Game/Chess/UI/UI_Main.SetMoveCount` (`self.MainUIRef`) (`/Game/Chess/Blueprints/BP_GameMode.GetMoveCount` (`self.GameModeRef`)))
      (`/Game/Chess/UI/UI_Main.SetPositionEvaluation` (`self.MainUIRef`) (`/Game/Chess/Blueprints/BP_GameMode.GetPositionEval` (`self.GameModeRef`)))
      (`/Game/Chess/UI/UI_Main.SetLatestMove` (`self.MainUIRef`) _color _latestmovenotation)
      (if (`/Game/Chess/Blueprints/BP_GameMode.GetChechkStatus` (`self.GameModeRef`))
        (`/Game/Chess/UI/UI_Main.SetMessage1` (`self.MainUIRef`) "InCheck!")
        (else
          (`/Game/Chess/UI/UI_Main.SetMessage1` (`self.MainUIRef`) "")))
      (`self.DisplayMessgaeBaseOnEndGame`)
      (return))))

(fn `UserConstructionScript`)
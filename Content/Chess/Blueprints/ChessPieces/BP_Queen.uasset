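; BP_Queen is the queen chess piece, defining which squares it highlights as possible moves.
; Its ShowPossibleMoves function clears existing highlights through the game mode, then calls diagonal, horizontal and vertical highlight helpers with the piece's color.
; The function returns the IsKing flag, and the event graph and construction script add no logic of their own.
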(fn `ShowPossibleMoves`
  (returns (IsKing :type Boolean))
  (bind _color (`self.Color`))
  (`|ExecutionSequence`
    (:`then_0`
      (`/Game/Chess/Blueprints/BP_GameMode.UnhighlightSquares` (`self.GameModeRef`)))
    (:`then_1`
      (`self.HighlightDiagonalSquares` _color))
    (:`then_2`
      (`self.HighlightHorizontalSquares` _color))
    (:`then_3`
      (`self.HighlightVertiaclSquares` _color))
    (:`then_4`
      (return (`self.IsKing`)))))

(fn `UserConstructionScript`
  (`parent.UserConstructionScript`))